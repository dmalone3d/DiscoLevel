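; Disco floor switch actor for the procedural tower that cycles its look at random while the game runs.
; On BeginPlay it starts a ColorChange event that picks one of four FloorTiles materials at random and applies it to the static mesh.
; The event then waits a second and calls itself, looping indefinitely.
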(event Custom|ColorChange
  (bind _staticmeshcomponent (Variables|Debug|GetStaticMeshComponent))
  (switch int (Math|Random|RandomIntegerinRange 0 3)
    (:Default
      (Rendering|Material|SetMaterial _staticmeshcomponent 0 "/Game/Team_Custom/3DAssets/FloorTiles.FloorTiles" :!label _label))
    (:0
      (goto _label))
    (:1
      (Rendering|Material|SetMaterial _staticmeshcomponent 0 "/Game/Team_Custom/3DAssets/FloorTiles2.FloorTiles2"))
    (:2
      (Rendering|Material|SetMaterial _staticmeshcomponent 0 "/Game/Team_Custom/3DAssets/FloorTiles3.FloorTiles3"))
    (:3
      (Rendering|Material|SetMaterial _staticmeshcomponent 0 "/Game/Team_Custom/3DAssets/FloorTiles4.FloorTiles4")))
  (Utilities|FlowControl|Delay 1.0)
  (CallFunction|ColorChange))

(event EventBeginPlay
  (CallFunction|ColorChange))

(fn ConstructionScript)