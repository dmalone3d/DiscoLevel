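; Disco floor puzzle where the player steps on nine switch tiles to reproduce a random lit pattern shown on paired screen panels.
; PuzzleRound randomises TargetArray and lights matching screens; each box overlap flip-flops its CheckArray entry and tile material.
; Most toggles then compare both arrays as joined strings, starting a new pattern on a match until the round limit prints completion.
; Switch states carry over between rounds, and BoolArray is filled but never read.
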(event OnComponentBeginOverlap(Box)
  (params (OverlappedComponent :type Primitive%20Component%20Object%20Reference) (OtherActor :type Actor%20Object%20Reference) (OtherComp :type Primitive%20Component%20Object%20Reference) (OtherBodyIndex :type Integer) (bFromSweep :type Boolean) (SweepResult :type Hit%20Result%20Structure%20%28by%20ref%29))
  (bind _switch (Variables|Default|GetSwitch))
  (bind _targetarray (Variables|Default|GetTargetArray))
  (bind _checkarray (Variables|Default|GetCheckArray))
  ;[1 1 1] Button1
  (Utilities|FlowControl|FlipFlop
    (:A
      (Utilities|Array|SetArrayElem _checkarray 0 "1")
      (Rendering|Material|SetMaterial _switch 0 "/Game/Team_Custom/3DAssets/FloorTiles4.FloorTiles4"))
    (:B
      (Utilities|Array|SetArrayElem _checkarray 0 (Utilities|String|ToString(Integer) (Variables|Default|GetFix%20int)))
      (Rendering|Material|SetMaterial _switch 0 "/Game/Team_Custom/3DAssets/FloorTiles5.FloorTiles5")))
  (if (Utilities|Enum|Equal(Enum) (Utilities|String|JoinStringArray (Variables|Default|GetTargetArray) " ") (Utilities|String|JoinStringArray (Variables|Default|GetCheckArray) " "))
    (bind _result (Math|Integer|IncrementInt (Variables|Default|GetRoundNum))
      (:%20%20
        (bind _output_get (Variables|Default|SetRoundNum _result))
        (if (== _output_get 4)
          (Development|PrintString "PUZZLECOMPLETE")
          (else
            (Rendering|Material|SetMaterial (Variables|Default|GetScreenP3) 0 "/Game/Team_Custom/3DAssets/FloorTiles5.FloorTiles5")
            (Variables|Default|SetIndex 0)
            (for (_ _array_index) _targetarray
              (Utilities|Array|SetArrayElem _targetarray _array_index (Utilities|String|ToString(Integer) (Variables|Default|GetFix%20int))))
            (CallFunction|PuzzleRound)
            (Development|PrintString (Utilities|String|ToString(Integer) (Variables|Default|GetRoundNum)))))))
    (else
      (Development|PrintString (Utilities|String|JoinStringArray (Variables|Default|GetCheckArray) " ")))))

(event OnComponentBeginOverlap(Box3)
  (params (OverlappedComponent :type Primitive%20Component%20Object%20Reference) (OtherActor :type Actor%20Object%20Reference) (OtherComp :type Primitive%20Component%20Object%20Reference) (OtherBodyIndex :type Integer) (bFromSweep :type Boolean) (SweepResult :type Hit%20Result%20Structure%20%28by%20ref%29))
  (bind _switch3 (Variables|Default|GetSwitch3))
  (bind _targetarray (Variables|Default|GetTargetArray))
  (bind _checkarray (Variables|Default|GetCheckArray))
  ;[1 1 1] Button4
  (Utilities|FlowControl|FlipFlop
    (:A
      (Utilities|Array|SetArrayElem _checkarray 3 "1")
      (Rendering|Material|SetMaterial _switch3 0 "/Game/Team_Custom/3DAssets/FloorTiles4.FloorTiles4"))
    (:B
      (Utilities|Array|SetArrayElem _checkarray 3 (Utilities|String|ToString(Integer) (Variables|Default|GetFix%20int)))
      (Rendering|Material|SetMaterial _switch3 0 "/Game/Team_Custom/3DAssets/FloorTiles5.FloorTiles5")))
  (if (Utilities|Enum|Equal(Enum) (Utilities|String|JoinStringArray (Variables|Default|GetTargetArray) " ") (Utilities|String|JoinStringArray (Variables|Default|GetCheckArray) " "))
    (bind _result (Math|Integer|IncrementInt (Variables|Default|GetRoundNum))
      (:%20%20
        (bind _output_get (Variables|Default|SetRoundNum _result))
        (if (== _output_get 4)
          (Development|PrintString "PUZZLECOMPLETE")
          (else
            (Rendering|Material|SetMaterial (Variables|Default|GetScreenP3) 0 "/Game/Team_Custom/3DAssets/FloorTiles5.FloorTiles5")
            (Variables|Default|SetIndex 0)
            (for (_ _array_index) _targetarray
              (Utilities|Array|SetArrayElem _targetarray _array_index (Utilities|String|ToString(Integer) (Variables|Default|GetFix%20int))))
            (CallFunction|PuzzleRound)
            (Development|PrintString (Utilities|String|ToString(Integer) (Variables|Default|GetRoundNum)))))))
    (else
      (Development|PrintString (Utilities|String|JoinStringArray (Variables|Default|GetCheckArray) " ")))))

(event OnComponentBeginOverlap(Box2)
  (params (OverlappedComponent :type Primitive%20Component%20Object%20Reference) (OtherActor :type Actor%20Object%20Reference) (OtherComp :type Primitive%20Component%20Object%20Reference) (OtherBodyIndex :type Integer) (bFromSweep :type Boolean) (SweepResult :type Hit%20Result%20Structure%20%28by%20ref%29))
  (bind _switch2 (Variables|Default|GetSwitch2))
  (bind _targetarray (Variables|Default|GetTargetArray))
  (bind _checkarray (Variables|Default|GetCheckArray))
  ;[1 1 1] Button3
  (Utilities|FlowControl|FlipFlop
    (:A
      (Utilities|Array|SetArrayElem _checkarray 2 "1")
      (Rendering|Material|SetMaterial _switch2 0 "/Game/Team_Custom/3DAssets/FloorTiles4.FloorTiles4"))
    (:B
      (Utilities|Array|SetArrayElem _checkarray 2 (Utilities|String|ToString(Integer) (Variables|Default|GetFix%20int)))
      (Rendering|Material|SetMaterial _switch2 0 "/Game/Team_Custom/3DAssets/FloorTiles5.FloorTiles5")))
  (if (Utilities|Enum|Equal(Enum) (Utilities|String|JoinStringArray (Variables|Default|GetTargetArray) " ") (Utilities|String|JoinStringArray (Variables|Default|GetCheckArray) " "))
    (bind _result (Math|Integer|IncrementInt (Variables|Default|GetRoundNum))
      (:%20%20
        (bind _output_get (Variables|Default|SetRoundNum _result))
        (if (== _output_get 4)
          (Development|PrintString "PUZZLECOMPLETE")
          (else
            (Rendering|Material|SetMaterial (Variables|Default|GetScreenP3) 0 "/Game/Team_Custom/3DAssets/FloorTiles5.FloorTiles5")
            (Variables|Default|SetIndex 0)
            (for (_ _array_index) _targetarray
              (Utilities|Array|SetArrayElem _targetarray _array_index (Utilities|String|ToString(Integer) (Variables|Default|GetFix%20int))))
            (CallFunction|PuzzleRound)
            (Development|PrintString (Utilities|String|ToString(Integer) (Variables|Default|GetRoundNum)))))))
    (else
      (Development|PrintString (Utilities|String|JoinStringArray (Variables|Default|GetCheckArray) " ")))))

(event OnComponentBeginOverlap(Box4)
  (params (OverlappedComponent :type Primitive%20Component%20Object%20Reference) (OtherActor :type Actor%20Object%20Reference) (OtherComp :type Primitive%20Component%20Object%20Reference) (OtherBodyIndex :type Integer) (bFromSweep :type Boolean) (SweepResult :type Hit%20Result%20Structure%20%28by%20ref%29))
  (bind _checkarray (Variables|Default|GetCheckArray))
  (bind _switch4 (Variables|Default|GetSwitch4))
  (bind _targetarray (Variables|Default|GetTargetArray))
  ;[1 1 1] Button5
  (Utilities|FlowControl|FlipFlop
    (:A
      (Utilities|Array|SetArrayElem _checkarray 4 "1")
      (Rendering|Material|SetMaterial _switch4 0 "/Game/Team_Custom/3DAssets/FloorTiles4.FloorTiles4"))
    (:B
      (Utilities|Array|SetArrayElem _checkarray 4 (Utilities|String|ToString(Integer) (Variables|Default|GetFix%20int)))
      (Rendering|Material|SetMaterial _switch4 0 "/Game/Team_Custom/3DAssets/FloorTiles5.FloorTiles5")))
  (if (Utilities|Enum|Equal(Enum) (Utilities|String|JoinStringArray (Variables|Default|GetTargetArray) " ") (Utilities|String|JoinStringArray (Variables|Default|GetCheckArray) " "))
    (bind _result (Math|Integer|IncrementInt (Variables|Default|GetRoundNum))
      (:%20%20
        (bind _output_get (Variables|Default|SetRoundNum _result))
        (if (== _output_get 4)
          (Development|PrintString "PUZZLECOMPLETE")
          (else
            (Rendering|Material|SetMaterial (Variables|Default|GetScreenP3) 0 "/Game/Team_Custom/3DAssets/FloorTiles5.FloorTiles5")
            (Variables|Default|SetIndex 0)
            (for (_ _array_index) _targetarray
              (Utilities|Array|SetArrayElem _targetarray _array_index (Utilities|String|ToString(Integer) (Variables|Default|GetFix%20int))))
            (CallFunction|PuzzleRound)
            (Development|PrintString (Utilities|String|ToString(Integer) (Variables|Default|GetRoundNum)))))))
    (else
      (Development|PrintString (Utilities|String|JoinStringArray (Variables|Default|GetCheckArray) " ")))))

(event OnComponentBeginOverlap(Box5)
  (params (OverlappedComponent :type Primitive%20Component%20Object%20Reference) (OtherActor :type Actor%20Object%20Reference) (OtherComp :type Primitive%20Component%20Object%20Reference) (OtherBodyIndex :type Integer) (bFromSweep :type Boolean) (SweepResult :type Hit%20Result%20Structure%20%28by%20ref%29))
  (bind _checkarray (Variables|Default|GetCheckArray))
  (bind _switch5 (Variables|Default|GetSwitch5))
  (bind _targetarray (Variables|Default|GetTargetArray))
  ;[1 1 1] Button6
  (Utilities|FlowControl|FlipFlop
    (:A
      (Utilities|Array|SetArrayElem _checkarray 5 "1")
      (Rendering|Material|SetMaterial _switch5 0 "/Game/Team_Custom/3DAssets/FloorTiles4.FloorTiles4"))
    (:B
      (Utilities|Array|SetArrayElem _checkarray 5 (Utilities|String|ToString(Integer) (Variables|Default|GetFix%20int)))
      (Rendering|Material|SetMaterial _switch5 0 "/Game/Team_Custom/3DAssets/FloorTiles5.FloorTiles5")))
  (if (Utilities|Enum|Equal(Enum) (Utilities|String|JoinStringArray (Variables|Default|GetTargetArray) " ") (Utilities|String|JoinStringArray (Variables|Default|GetCheckArray) " "))
    (bind _result (Math|Integer|IncrementInt (Variables|Default|GetRoundNum))
      (:%20%20
        (bind _output_get (Variables|Default|SetRoundNum _result))
        (if (== _output_get 4)
          (Development|PrintString "PUZZLECOMPLETE")
          (else
            (Rendering|Material|SetMaterial (Variables|Default|GetScreenP3) 0 "/Game/Team_Custom/3DAssets/FloorTiles5.FloorTiles5")
            (Variables|Default|SetIndex 0)
            (for (_ _array_index) _targetarray
              (Utilities|Array|SetArrayElem _targetarray _array_index (Utilities|String|ToString(Integer) (Variables|Default|GetFix%20int))))
            (CallFunction|PuzzleRound)
            (Development|PrintString (Utilities|String|ToString(Integer) (Variables|Default|GetRoundNum)))))))
    (else
      (Development|PrintString (Utilities|String|JoinStringArray (Variables|Default|GetCheckArray) " ")))))

(event OnComponentBeginOverlap(Box6)
  (params (OverlappedComponent :type Primitive%20Component%20Object%20Reference) (OtherActor :type Actor%20Object%20Reference) (OtherComp :type Primitive%20Component%20Object%20Reference) (OtherBodyIndex :type Integer) (bFromSweep :type Boolean) (SweepResult :type Hit%20Result%20Structure%20%28by%20ref%29))
  (bind _checkarray (Variables|Default|GetCheckArray))
  (bind _switch6 (Variables|Default|GetSwitch6))
  (bind _targetarray (Variables|Default|GetTargetArray))
  ;[1 1 1] Button7
  (Utilities|FlowControl|FlipFlop
    (:A
      (Utilities|Array|SetArrayElem _checkarray 6 "1")
      (Rendering|Material|SetMaterial _switch6 0 "/Game/Team_Custom/3DAssets/FloorTiles4.FloorTiles4"))
    (:B
      (Utilities|Array|SetArrayElem _checkarray 6 (Utilities|String|ToString(Integer) (Variables|Default|GetFix%20int)))
      (Rendering|Material|SetMaterial _switch6 0 "/Game/Team_Custom/3DAssets/FloorTiles5.FloorTiles5")))
  (if (Utilities|Enum|Equal(Enum) (Utilities|String|JoinStringArray (Variables|Default|GetTargetArray) " ") (Utilities|String|JoinStringArray (Variables|Default|GetCheckArray) " "))
    (bind _result (Math|Integer|IncrementInt (Variables|Default|GetRoundNum))
      (:%20%20
        (bind _output_get (Variables|Default|SetRoundNum _result))
        (if (== _output_get 4)
          (Development|PrintString "PUZZLECOMPLETE")
          (else
            (Rendering|Material|SetMaterial (Variables|Default|GetScreenP3) 0 "/Game/Team_Custom/3DAssets/FloorTiles5.FloorTiles5")
            (Variables|Default|SetIndex 0)
            (for (_ _array_index) _targetarray
              (Utilities|Array|SetArrayElem _targetarray _array_index (Utilities|String|ToString(Integer) (Variables|Default|GetFix%20int))))
            (CallFunction|PuzzleRound)
            (Development|PrintString (Utilities|String|ToString(Integer) (Variables|Default|GetRoundNum)))))))
    (else
      (Development|PrintString (Utilities|String|JoinStringArray (Variables|Default|GetCheckArray) " ")))))

(event OnComponentBeginOverlap(Box1)
  (params (OverlappedComponent :type Primitive%20Component%20Object%20Reference) (OtherActor :type Actor%20Object%20Reference) (OtherComp :type Primitive%20Component%20Object%20Reference) (OtherBodyIndex :type Integer) (bFromSweep :type Boolean) (SweepResult :type Hit%20Result%20Structure%20%28by%20ref%29))
  (bind _switch1 (Variables|Default|GetSwitch1))
  (bind _targetarray (Variables|Default|GetTargetArray))
  (bind _checkarray (Variables|Default|GetCheckArray))
  ;[1 1 1] Button2
  (Utilities|FlowControl|FlipFlop
    (:A
      (Utilities|Array|SetArrayElem _checkarray 1 "1")
      (Rendering|Material|SetMaterial _switch1 0 "/Game/Team_Custom/3DAssets/FloorTiles4.FloorTiles4"))
    (:B
      (Utilities|Array|SetArrayElem _checkarray 1 (Utilities|String|ToString(Integer) (Variables|Default|GetFix%20int)))
      (Rendering|Material|SetMaterial _switch1 0 "/Game/Team_Custom/3DAssets/FloorTiles5.FloorTiles5")))
  (if (Utilities|Enum|Equal(Enum) (Utilities|String|JoinStringArray (Variables|Default|GetTargetArray) " ") (Utilities|String|JoinStringArray (Variables|Default|GetCheckArray) " "))
    (bind _result (Math|Integer|IncrementInt (Variables|Default|GetRoundNum))
      (:%20%20
        (bind _output_get (Variables|Default|SetRoundNum _result))
        (if (== _output_get 4)
          (Development|PrintString "PUZZLECOMPLETE")
          (else
            (Rendering|Material|SetMaterial (Variables|Default|GetScreenP3) 0 "/Game/Team_Custom/3DAssets/FloorTiles5.FloorTiles5")
            (Variables|Default|SetIndex 0)
            (for (_ _array_index) _targetarray
              (Utilities|Array|SetArrayElem _targetarray _array_index (Utilities|String|ToString(Integer) (Variables|Default|GetFix%20int))))
            (CallFunction|PuzzleRound)
            (Development|PrintString (Utilities|String|ToString(Integer) (Variables|Default|GetRoundNum)))))))
    (else
      (Development|PrintString (Utilities|String|JoinStringArray (Variables|Default|GetCheckArray) " ")))))

(event OnComponentBeginOverlap(Box7)
  (params (OverlappedComponent :type Primitive%20Component%20Object%20Reference) (OtherActor :type Actor%20Object%20Reference) (OtherComp :type Primitive%20Component%20Object%20Reference) (OtherBodyIndex :type Integer) (bFromSweep :type Boolean) (SweepResult :type Hit%20Result%20Structure%20%28by%20ref%29))
  (bind _checkarray (Variables|Default|GetCheckArray))
  (bind _switch7 (Variables|Default|GetSwitch7))
  (bind _targetarray (Variables|Default|GetTargetArray))
  ;[1 1 1] Button8
  (Utilities|FlowControl|FlipFlop
    (:A
      (Utilities|Array|SetArrayElem _checkarray 7 "1")
      (Rendering|Material|SetMaterial _switch7 0 "/Game/Team_Custom/3DAssets/FloorTiles4.FloorTiles4"))
    (:B
      (Utilities|Array|SetArrayElem _checkarray 7 (Utilities|String|ToString(Integer) (Variables|Default|GetFix%20int)))
      (Rendering|Material|SetMaterial _switch7 0 "/Game/Team_Custom/3DAssets/FloorTiles5.FloorTiles5")))
  (if (Utilities|Enum|Equal(Enum) (Utilities|String|JoinStringArray (Variables|Default|GetTargetArray) " ") (Utilities|String|JoinStringArray (Variables|Default|GetCheckArray) " "))
    (bind _result (Math|Integer|IncrementInt (Variables|Default|GetRoundNum))
      (:%20%20
        (bind _output_get (Variables|Default|SetRoundNum _result))
        (if (== _output_get 4)
          (Development|PrintString "PUZZLECOMPLETE")
          (else
            (Rendering|Material|SetMaterial (Variables|Default|GetScreenP3) 0 "/Game/Team_Custom/3DAssets/FloorTiles5.FloorTiles5")
            (Variables|Default|SetIndex 0)
            (for (_ _array_index) _targetarray
              (Utilities|Array|SetArrayElem _targetarray _array_index (Utilities|String|ToString(Integer) (Variables|Default|GetFix%20int))))
            (CallFunction|PuzzleRound)
            (Development|PrintString (Utilities|String|ToString(Integer) (Variables|Default|GetRoundNum)))))))
    (else
      (Development|PrintString (Utilities|String|JoinStringArray (Variables|Default|GetCheckArray) " ")))))

(event OnComponentBeginOverlap(Box8)
  (params (OverlappedComponent :type Primitive%20Component%20Object%20Reference) (OtherActor :type Actor%20Object%20Reference) (OtherComp :type Primitive%20Component%20Object%20Reference) (OtherBodyIndex :type Integer) (bFromSweep :type Boolean) (SweepResult :type Hit%20Result%20Structure%20%28by%20ref%29))
  (bind _checkarray (Variables|Default|GetCheckArray))
  (bind _switch8 (Variables|Default|GetSwitch8))
  (bind _targetarray (Variables|Default|GetTargetArray))
  ;[1 1 1] Button9
  (Utilities|FlowControl|FlipFlop
    (:A
      (Utilities|Array|SetArrayElem _checkarray 8 "1")
      (Rendering|Material|SetMaterial _switch8 0 "/Game/Team_Custom/3DAssets/FloorTiles4.FloorTiles4"))
    (:B
      (Utilities|Array|SetArrayElem _checkarray 8 (Utilities|String|ToString(Integer) (Variables|Default|GetFix%20int)))
      (Rendering|Material|SetMaterial _switch8 0 "/Game/Team_Custom/3DAssets/FloorTiles5.FloorTiles5")))
  (if (Utilities|Enum|Equal(Enum) (Utilities|String|JoinStringArray (Variables|Default|GetTargetArray) " ") (Utilities|String|JoinStringArray (Variables|Default|GetCheckArray) " "))
    (bind _result (Math|Integer|IncrementInt (Variables|Default|GetRoundNum))
      (:%20%20
        (bind _output_get (Variables|Default|SetRoundNum _result))
        (if (== _output_get 4)
          (Development|PrintString "PUZZLECOMPLETE")
          (else
            (Rendering|Material|SetMaterial (Variables|Default|GetScreenP3) 0 "/Game/Team_Custom/3DAssets/FloorTiles5.FloorTiles5")
            (Variables|Default|SetIndex 0)
            (for (_ _array_index) _targetarray
              (Utilities|Array|SetArrayElem _targetarray _array_index (Utilities|String|ToString(Integer) (Variables|Default|GetFix%20int))))
            (CallFunction|PuzzleRound)
            (Development|PrintString (Utilities|String|ToString(Integer) (Variables|Default|GetRoundNum)))))))
    (else
      (Development|PrintString (Utilities|String|JoinStringArray (Variables|Default|GetCheckArray) " ")))))

(event Custom|PuzzleRound
  (bind _returnvalue (Math|Random|RandomInteger 2))
  (bind _targetarray (Variables|Default|GetTargetArray))
  (bind _returnvalue_2 (Utilities|String|ToString(Integer) _returnvalue))
  (for _array_element _targetarray
    (Utilities|Array|SetArrayElem _targetarray (Variables|Default|GetIndex) _returnvalue_2)
    (Utilities|Array|SetArrayElem (Variables|Default|GetBoolArray) (Variables|Default|GetIndex) (Math|Conversions|ToBoolean(Integer) (Math|Conversions|ToInteger(Byte) _returnvalue_2)))
    (Variables|Default|SetIndex (+ (Variables|Default|GetIndex) 1)))
  (Development|PrintString (Utilities|String|JoinStringArray _targetarray " "))
  ;[1 1 1] Screen Lighting
  (Utilities|FlowControl|Sequence
    (:then_0
      (if (Utilities|Enum|Equal(Enum) (Utilities|Array|Get(acopy) (Variables|Default|GetTargetArray)) "1")
        (Rendering|Material|SetMaterial (Variables|Default|GetScreenP) 0 "/Game/Team_Custom/3DAssets/FloorTiles4.FloorTiles4")))
    (:then_1
      (if (Utilities|Enum|Equal(Enum) (Utilities|Array|Get(acopy) (Variables|Default|GetTargetArray) 1) "1")
        (Rendering|Material|SetMaterial (Variables|Default|GetScreenP10) 0 "/Game/Team_Custom/3DAssets/FloorTiles4.FloorTiles4")))
    (:then_2
      (if (Utilities|Enum|Equal(Enum) (Utilities|Array|Get(acopy) (Variables|Default|GetTargetArray) 2) "1")
        (Rendering|Material|SetMaterial (Variables|Default|GetScreenP11) 0 "/Game/Team_Custom/3DAssets/FloorTiles4.FloorTiles4")))
    (:then_3
      (if (Utilities|Enum|Equal(Enum) (Utilities|Array|Get(acopy) (Variables|Default|GetTargetArray) 3) "1")
        (Rendering|Material|SetMaterial (Variables|Default|GetScreenP3) 0 "/Game/Team_Custom/3DAssets/FloorTiles4.FloorTiles4")))
    (:then_4
      (if (Utilities|Enum|Equal(Enum) (Utilities|Array|Get(acopy) (Variables|Default|GetTargetArray) 4) "1")
        (Rendering|Material|SetMaterial (Variables|Default|GetScreenP13) 0 "/Game/Team_Custom/3DAssets/FloorTiles4.FloorTiles4")))
    (:then_5
      (if (Utilities|Enum|Equal(Enum) (Utilities|Array|Get(acopy) (Variables|Default|GetTargetArray) 5) "1")
        (Rendering|Material|SetMaterial (Variables|Default|GetScreenP14) 0 "/Game/Team_Custom/3DAssets/FloorTiles4.FloorTiles4")))
    (:then_6
      (if (Utilities|Enum|Equal(Enum) (Utilities|Array|Get(acopy) (Variables|Default|GetTargetArray) 6) "1")
        (Rendering|Material|SetMaterial (Variables|Default|GetScreenP15) 0 "/Game/Team_Custom/3DAssets/FloorTiles4.FloorTiles4")))
    (:then_7
      (if (Utilities|Enum|Equal(Enum) (Utilities|Array|Get(acopy) (Variables|Default|GetTargetArray) 7) "1")
        (Rendering|Material|SetMaterial (Variables|Default|GetScreenP7) 0 "/Game/Team_Custom/3DAssets/FloorTiles4.FloorTiles4")))
    (:then_8
      (if (Utilities|Enum|Equal(Enum) (Utilities|Array|Get(acopy) (Variables|Default|GetTargetArray) 8) "1")
        (Rendering|Material|SetMaterial (Variables|Default|GetScreenP17) 0 "/Game/Team_Custom/3DAssets/FloorTiles4.FloorTiles4")))))

(event EventBeginPlay
  (CallFunction|PuzzleRound)
  (Development|PrintString (Utilities|String|ToString(Integer) (Variables|Default|GetRoundNum))))

(fn ConstructionScript)