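; Ballet_New is a pad-and-light memory puzzle that rolls a random three-step combination of 1 to 3 on BeginPlay.
; Overlapping the three numbered pads writes their digits into successive slots of the player's attempt.
; The green pad compares both sequences as joined strings, destroying several mesh and effect components on a match.
; A mismatch resets the attempt and replays the combination through timed spotlight flashes, with debug prints exposing the answer.
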(event OnComponentBeginOverlap(Pad1)
  (params (OverlappedComponent :type Primitive%20Component%20Object%20Reference) (OtherActor :type Actor%20Object%20Reference) (OtherComp :type Primitive%20Component%20Object%20Reference) (OtherBodyIndex :type Integer) (bFromSweep :type Boolean) (SweepResult :type Hit%20Result%20Structure%20%28by%20ref%29))
  ;[1 1 1] Adds "1" to Order Compare
  (Utilities|Array|SetArrayElem (Variables|Default|GetOrderCompare) (Variables|Default|GetOrder%20Index) (Utilities|Array|Get(acopy) (Variables|Default|GetPad%20Number)))
  (Math|Integer|IncrementInt (Variables|Default|GetOrder%20Index)))

(event OnComponentBeginOverlap(Pad2)
  (params (OverlappedComponent :type Primitive%20Component%20Object%20Reference) (OtherActor :type Actor%20Object%20Reference) (OtherComp :type Primitive%20Component%20Object%20Reference) (OtherBodyIndex :type Integer) (bFromSweep :type Boolean) (SweepResult :type Hit%20Result%20Structure%20%28by%20ref%29))
  ;[1 1 1] Adds "2" to to Order Compare
  (Utilities|Array|SetArrayElem (Variables|Default|GetOrderCompare) (Variables|Default|GetOrder%20Index) (Utilities|Array|Get(acopy) (Variables|Default|GetPad%20Number) 1))
  (Math|Integer|IncrementInt (Variables|Default|GetOrder%20Index)))

(event OnComponentBeginOverlap(Pad3)
  (params (OverlappedComponent :type Primitive%20Component%20Object%20Reference) (OtherActor :type Actor%20Object%20Reference) (OtherComp :type Primitive%20Component%20Object%20Reference) (OtherBodyIndex :type Integer) (bFromSweep :type Boolean) (SweepResult :type Hit%20Result%20Structure%20%28by%20ref%29))
  ;[1 1 1] Adds "3" to Order Compare
  (Utilities|Array|SetArrayElem (Variables|Default|GetOrderCompare) (Variables|Default|GetOrder%20Index) (Utilities|Array|Get(acopy) (Variables|Default|GetPad%20Number) 2))
  (Math|Integer|IncrementInt (Variables|Default|GetOrder%20Index)))

(event OnComponentBeginOverlap(GreenPad)
  (params (OverlappedComponent :type Primitive%20Component%20Object%20Reference) (OtherActor :type Actor%20Object%20Reference) (OtherComp :type Primitive%20Component%20Object%20Reference) (OtherBodyIndex :type Integer) (bFromSweep :type Boolean) (SweepResult :type Hit%20Result%20Structure%20%28by%20ref%29))
  (bind _ordercompare (Variables|Default|GetOrderCompare))
  (bind _returnvalue (Utilities|String|JoinStringArray _ordercompare ""))
  ;[1 1 1] Compares Order
  (Development|PrintString _returnvalue)
  (if (Utilities|Enum|Equal(Enum) (Utilities|String|JoinStringArray (Variables|Default|GetOrder) "") _returnvalue)
    (Development|PrintString "PUZZLE SOLVED" true true "(R=0.000000,G=1.000000,B=0.102894,A=1.000000)" 1e+01)
    (Components|DestroyComponent (Variables|Default|GetStaticMesh))
    (else
      (Variables|Default|SetOrder%20Index 0)
      (Utilities|Array|Clear _ordercompare)
      (for _index (range 0 2)
        (Utilities|Array|Add (Variables|Default|GetOrderCompare) (Utilities|String|ToString(Integer) (Variables|Default|GetOrder%20Index))))
      (Development|PrintString "Cleared array and reshow order" true true "(R=1.000000,G=0.000000,B=0.057555,A=1.000000)")
      (Development|PrintString (Utilities|String|Append "Combination Set:" (Utilities|String|JoinStringArray (Variables|Default|GetOrder) "")) true true "(R=1.000000,G=0.000000,B=0.057555,A=1.000000)")
      (CallFunction|ShowLIghts))))

(event Custom|Show%20LIghts
  (bind _variable (|TemporaryVariable))
  (bind _order (Variables|Default|GetOrder))
  (bind _spotlight1 (Variables|Default|GetSpotLight1))
  (bind _spotlight (Variables|Default|GetSpotLight))
  (bind _spotlight2 (Variables|Default|GetSpotLight2))
  (bind _item (Utilities|Array|Get(acopy) _order _variable))
  (bind _array (Utilities|Array|MakeArray 0 _spotlight1 _spotlight _spotlight2))
  (bind _returnvalue (Math|Conversions|ToInteger(Byte) _item))
  (bind _item_2 (Utilities|Array|Get(acopy) _array _returnvalue))
  (|Assign _variable 0)
  (if (<= _variable 2) :!label _label
    (Rendering|Components|Light|SetIntensity _item_2 5e+03)
    (Utilities|FlowControl|Delay 2.0)
    (Rendering|Components|Light|SetIntensity _item_2 0.0)
    (Utilities|FlowControl|Delay 1.0)
    (|Assign _variable (+ _variable 1))
    (goto _label)))

(event EventBeginPlay
  (bind _order (Variables|Default|GetOrder))
  ;[1 1 1] Sets solution at start
  (for _index (range 0 2)
    (Utilities|Array|SetArrayElem _order _index (Utilities|String|ToString(Integer) (Math|Random|RandomIntegerinRange 1 3))))
  (Development|PrintString (Utilities|String|Append "Combination Set:" (Utilities|String|JoinStringArray _order "")) true true "(R=0.000000,G=0.660000,B=1.000000,A=1.000000)" 5.0))

(fn ConstructionScript)