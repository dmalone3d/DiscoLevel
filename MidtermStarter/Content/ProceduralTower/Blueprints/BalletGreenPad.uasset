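; BalletGreenPad is a pad actor that checks a combination puzzle, judging by its folder in a procedural tower.
; On BeginPlay it fills Order with three random digits as strings and prints the combination.
; On overlap it joins Order and OrderCompare into strings and compares them, printing a solved or failed message.
; Nothing here fills OrderCompare, and the failure branch only prints that it cleared the array, without clearing it.
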(event EventBeginPlay
  (bind _order (Variables|Default|GetOrder))
  (for _index (range 0 2)
    (Utilities|Array|SetArrayElem _order _index (Utilities|String|ToString(Integer) (Math|Random|RandomIntegerinRange 1 3))))
  (Development|PrintString (Utilities|String|Append "Combination Set:" (Utilities|String|JoinStringArray _order "")) true true "(R=0.000000,G=0.660000,B=1.000000,A=1.000000)" 5.0))

(event Collision|EventActorBeginOverlap
  (params (OtherActor :type Actor%20Object%20Reference))
  (bind _ordercompare (Variables|Default|GetOrderCompare))
  (bind _returnvalue (Utilities|String|JoinStringArray _ordercompare ""))
  (Development|PrintString _returnvalue)
  (if (Utilities|Enum|Equal(Enum) (Utilities|String|JoinStringArray (Variables|Default|GetOrder) "") _returnvalue)
    (Development|PrintString "PUZZLE SOLVED" true true "(R=0.000000,G=1.000000,B=0.102894,A=1.000000)")
    (else
      (Development|PrintString "Cleared array and reshow order" true true "(R=1.000000,G=0.000000,B=0.057555,A=1.000000)"))))

(fn ConstructionScript)